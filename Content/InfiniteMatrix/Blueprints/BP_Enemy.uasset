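; BP_Enemy is a randomly placed enemy that the player can collide with or shoot.
; On BeginPlay, one in six instances survives and shifts randomly in Y and Z, while the rest destroy themselves.
; Mesh overlap with BP_Player cuts health, updates its progress bar and destroys the enemy, showing restart and stopping forward speed at zero health.
; Overlap with BP_Projectile destroys the enemy, increments player score and shows a hitmarker widget.
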(event OnComponentBeginOverlap(StaticMesh)
  (params (OverlappedComponent :type Primitive%20Component%20Object%20Reference) (OtherActor :type Actor%20Object%20Reference) (OtherComp :type Primitive%20Component%20Object%20Reference) (OtherBodyIndex :type Integer) (bFromSweep :type Boolean) (SweepResult :type Hit%20Result%20Structure%20%28by%20ref%29))
  (bind _asbp_player (Utilities|Casting|CastToBP_Player OtherActor)
    (:then
      (bind _output_get (Variables|/Game/InfiniteMatrix/Blueprints/BP_Player.BP_Player_C|Sethealth _asbp_player (- (Variables|/Game/InfiniteMatrix/Blueprints/BP_Player.BP_Player_C|Gethealth _asbp_player) 25)))
      (Variables|/Script/UMG.ProgressBar|SetPercent (Variables|/Game/InfiniteMatrix/UI/Health_Bar.Health_Bar_C|GetProgressBar_1 (Variables|/Game/InfiniteMatrix/Blueprints/BP_Player.BP_Player_C|Gethealth_widget _asbp_player)) (/ (Math|Conversions|ToFloat(Integer) _output_get) 1e+02))
      (Actor|DestroyActor)
      (if (== 0 _output_get)
        (Default|DisplayRestart _asbp_player)
        (Variables|/Game/InfiniteMatrix/Blueprints/BP_Player.BP_Player_C|SetForwardSpeed _asbp_player 0.0)))
    (:CastFailed
      (Utilities|Casting|CastToBP_Projectile OtherActor)
      (Actor|DestroyActor)
      (bind _asbp_player_2 (Utilities|Casting|CastToBP_Player (Game|Player|GetPlayerPawn 0)))
      (Variables|/Game/InfiniteMatrix/Blueprints/BP_Player.BP_Player_C|Setscore _asbp_player_2 (+ 1 (Variables|/Game/InfiniteMatrix/Blueprints/BP_Player.BP_Player_C|Getscore _asbp_player_2)))
      (bind _returnvalue (UserInterface|CreateWidget "/Game/InfiniteMatrix/UI/Hitmarker.Hitmarker_C"))
      (UserInterface|Viewport|AddtoViewport _returnvalue 0))))

(event EventBeginPlay
  (if (== 0 (Math|Random|RandomInteger 6))
    (Transformation|AddActorWorldOffset (Math|Vector|MakeVector 0.0 (Math|Random|RandomFloatinRange -2.5e+02 2.5e+02) (Math|Random|RandomFloatinRange -2.5e+02 2.5e+02)))
    (else
      (Actor|DestroyActor))))

(event Collision|EventActorBeginOverlap
  (params (OtherActor :type Actor%20Object%20Reference)))

(event EventTick
  (params (DeltaSeconds :type Float%20%28single-precision%29)))

(fn ConstructionScript)